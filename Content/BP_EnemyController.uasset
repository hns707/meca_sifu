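; Enemy AI controller that runs the BT_Enemy behavior tree and feeds it sightings of the player character.
; When perception updates on a living ThirdPersonCharacter_Sifu, a successful sense writes it to the PlayerRef blackboard key.
; A failed sense stores the stimulus location in LastSeenPos and clears PlayerRef.
; A ResetPlayerRef event also clears the target and prints a debug string.
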(event `self.ReceiveBeginPlay`
  (`self.RunBehaviorTree` "/Game/BT_Enemy.BT_Enemy"))

(event `self.AIPerception.OnTargetPerceptionUpdated`
  (params (Actor :type "Actor Object Reference") (Stimulus :type "AIStimulus Structure"))
  (bind _returnvalue (`AIBlueprintHelperLibrary.GetBlackboard` null))
  (bind _returnvalue_2 (`KismetStringLibrary.Conv_StringToName` "PlayerRef"))
  (bind _asthird_person_character_sifu (cast `/Game/ThirdPersonCharacter_Sifu` Actor))
  (if (`/Game/ThirdPersonCharacter_Sifu.isAlive` _asthird_person_character_sifu)
    (if Stimulus_bSuccessfullySensed
      (`BlackboardComponent.SetValueAsObject` _returnvalue _returnvalue_2 _asthird_person_character_sifu)
      (else
        (`BlackboardComponent.SetValueAsVector` _returnvalue (`KismetStringLibrary.Conv_StringToName` "LastSeenPos") Stimulus_StimulusLocation)
        (`BlackboardComponent.ClearValue` _returnvalue _returnvalue_2)))))

(event `ResetPlayerRef`
  (`BlackboardComponent.ClearValue` (`AIBlueprintHelperLibrary.GetBlackboard` null) (`KismetStringLibrary.Conv_StringToName` "PlayerRef"))
  (`KismetSystemLibrary.PrintString` "Hello"))

(fn `UserConstructionScript`)