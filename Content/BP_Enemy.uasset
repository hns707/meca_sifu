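; Enemy actor with health, a health bar shown above it, and ragdoll death.
; A sphere overlap shows the bar only while the Sifu player character is inside, and Tick turns it to face the camera.
; AnyDamage lowers Health and updates the bar assuming a maximum of 100.
; At exactly zero health it enables mesh physics, disables capsule collision, detaches the controller and calls the widget's FadeIn.
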(event `self.ReceiveBeginPlay`
  (`SceneComponent.SetVisibility` (`self.HPBar`) false false))

(event `self.ReceiveAnyDamage`
  (params (Damage :type "Float (single-precision)") (DamageType :type "DamageType Object Reference") (InstigatedBy :type "Controller Object Reference") (DamageCauser :type "Actor Object Reference"))
  (bind _mesh (`self.Mesh`))
  (bind _output_get (set `self.Health` (`KismetMathLibrary.FTrunc` (- (`self.Health`) Damage))))
  (`ProgressBar.SetPercent` (`/Game/UI_EnemyHealthBar.HpBar` (cast `/Game/UI_EnemyHealthBar` (`WidgetComponent.GetWidget` (`self.HPBar`)) :!pure true)) (/ (`self.Health`) (`KismetMathLibrary.Conv_IntToDouble` 100)))
  (if (== _output_get 0)
    (`PrimitiveComponent.SetSimulatePhysics` _mesh true)
    (`PrimitiveComponent.SetCollisionEnabled` (`self.CapsuleComponent`) "NoCollision")
    (`self.DetachFromControllerPendingDestroy`)
    (`SkeletalMeshComponent.SetAnimationMode` _mesh "AnimationSingleNode")
    (`/Game/UI_EnemyHealthBar.FadeIn` (cast `/Game/UI_EnemyHealthBar` (`WidgetComponent.GetWidget` (`self.HPBar`)) :!pure true))))

(event `self.ReceiveTick`
  (params (DeltaSeconds :type "Float (single-precision)"))
  (`self.HpBar_Update`))

(event `HpBar_Update`
  (bind (_returnvalue_roll _returnvalue_pitch _returnvalue_yaw) (`KismetMathLibrary.BreakRotator` (`PlayerCameraManager.GetCameraRotation` (`GameplayStatics.GetPlayerCameraManager` 0))))
  (`SceneComponent.K2_SetWorldRotation` (`self.HPBar`) (`KismetMathLibrary.MakeRotator` _returnvalue_roll (* _returnvalue_pitch -1.0) (+ _returnvalue_yaw 180.0)) false false))

(event `self.Sphere.OnComponentBeginOverlap`
  (params (OverlappedComponent :type "PrimitiveComponent Object Reference") (OtherActor :type "Actor Object Reference") (OtherComp :type "PrimitiveComponent Object Reference") (OtherBodyIndex :type Integer) (bFromSweep :type Boolean) (SweepResult :type "HitResult Structure (by ref)"))
  (cast `/Game/ThirdPersonCharacter_Sifu` OtherActor)
  (`SceneComponent.SetVisibility` (`self.HPBar`) true false))

(event `self.Sphere.OnComponentEndOverlap`
  (params (OverlappedComponent :type "PrimitiveComponent Object Reference") (OtherActor :type "Actor Object Reference") (OtherComp :type "PrimitiveComponent Object Reference") (OtherBodyIndex :type Integer))
  (cast `/Game/ThirdPersonCharacter_Sifu` OtherActor)
  (`SceneComponent.SetVisibility` (`self.HPBar`) false false))

(fn `UserConstructionScript`)